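; Player controller for the TPS start screen, which shows the start menu widget and hosts LAN games.
; BeginPlay creates a save settings object, adds the widget and enables mouse input for game and UI.
; OpenLobby, on authority only, creates a two-slot LAN session and opens the Lobby level as a listen server.
; SaveIP and LoadIP persist the last IP address through the save game slot.
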(event `self.ReceiveBeginPlay`
  (bind _returnvalue (`GameplayStatics.CreateSaveGameObject` "/Game/Blueprints/TPSStart/BP_SaveSettings.BP_SaveSettings_C"))
  (set `self.SaveSettingsInstance` _returnvalue)
  (bind _returnvalue_2 (`|CreateWidget` "/Game/Blueprints/TPSStart/TPSStartWidget.TPSStartWidget_C"))
  (set `self.TPSStartWidget` _returnvalue_2)
  (`UserWidget.AddToViewport` (`self.TPSStartWidget`) 0)
  (set `self.bShowMouseCursor` true)
  (`WidgetBlueprintLibrary.SetInputMode_GameAndUIEx` self null))

(event `OpenLobby`
  (`/Engine/EditorBlueprintResources/ActorMacros.Switch Has Authority`
    (:`Authority`
      (`CreateSessionCallbackProxy.CreateSession` self 2 true
        (:`OnSuccess`
          (`GameplayStatics.OpenLevel` "Lobby" true "listen"))))))

(fn `LoadIP`
  (returns (LastIPAddress :type String))
  (bind _returnvalue (`GameplayStatics.LoadGameFromSlot` (`/Game/Blueprints/TPSStart/BP_SaveSettings.SaveSlotName` (stale _output_get))))
  (bind _asbp_save_settings (cast `/Game/Blueprints/TPSStart/BP_SaveSettings` _returnvalue))
  (`/Engine/EditorBlueprintResources/StandardMacros.IsValid` _asbp_save_settings
    (:`Is Valid`
      (bind _output_get (set `self.SaveSettingsInstance` _asbp_save_settings))
      (return (`/Game/Blueprints/TPSStart/BP_SaveSettings.LastIPAddress` _output_get)))))

(fn `SaveIP`
  (params (NewIP :type String))
  (bind _savesettingsinstance (`self.SaveSettingsInstance`))
  (set `/Game/Blueprints/TPSStart/BP_SaveSettings.LastIPAddress` NewIP _savesettingsinstance)
  (`GameplayStatics.SaveGameToSlot` _savesettingsinstance (`/Game/Blueprints/TPSStart/BP_SaveSettings.SaveSlotName` _savesettingsinstance)))

(fn `UserConstructionScript`)