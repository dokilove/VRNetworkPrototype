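; BP_StartSwitch is a switch for the VR start area that sends the player on to the lobby when activated.
; Its DoSwitchAction event prints a debug "Hello", casts player controller 0 to BP_VRStartPC and calls OpenLobby on it if valid.
; BeginPlay, overlap and Tick are disabled stubs, and nothing in this graph triggers the switch action.
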(event `self.DoSwitchAction`
  (params (NewParam :type Boolean))
  (`KismetSystemLibrary.PrintString` "Hello")
  (bind _asbp_vrstart_pc (cast `/Game/Blueprints/VRStart/BP_VRStartPC` (`GameplayStatics.GetPlayerController` 0)))
  (`/Engine/EditorBlueprintResources/StandardMacros.IsValid` _asbp_vrstart_pc
    (:`Is Valid`
      (`/Game/Blueprints/VRStart/BP_VRStartPC.OpenLobby` _asbp_vrstart_pc))))

(fn `UserConstructionScript`
  (`parent.UserConstructionScript`))