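; BP_VRStartPC is the VR start controller that presents a start switch to the player and provides the event for hosting the lobby.
; On BeginPlay it spawns BP_StartSwitch a short distance in front of the BP_VRPawn camera and attaches it there, so the switch follows the head with its rotation snapped to the camera.
; OpenLobby loads the Lobby level as a listen server; its caller is outside this Blueprint.
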(event `self.ReceiveBeginPlay`
  (bind _asbp_vrpawn (cast `/Game/Blueprints/Character/VR/BP_VRPawn` (`GameplayStatics.GetPlayerPawn` 0)))
  (`/Engine/EditorBlueprintResources/StandardMacros.IsValid` _asbp_vrpawn
    (:`Is Valid`
      (bind _camera (`/Game/Blueprints/Character/VR/BP_VRPawn.Camera` _asbp_vrpawn))
      (bind _returnvalue (`|SpawnActorFromClass` "/Game/Blueprints/VRStart/BP_StartSwitch.BP_StartSwitch_C" (`KismetMathLibrary.MakeTransform` (+ (`SceneComponent.K2_GetComponentLocation` _camera) (* (`SceneComponent.GetForwardVector` _camera) 60.0))) "Undefined" "OverrideRootScale" _asbp_vrpawn null))
      (`self.K2_AttachToComponent` _returnvalue _camera "None" "KeepWorld" "SnapToTarget" "KeepRelative" true))))

(event `OpenLobby`
  (`GameplayStatics.OpenLevel` "Lobby" true "listen"))

(fn `UserConstructionScript`)