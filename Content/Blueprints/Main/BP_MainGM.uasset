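; Main game mode that spawns and possesses a pawn for each joining player, pairing one VR player with non-VR characters.
; On PostLogin, PlayerIndex selects class and transform: the first gets BP_VRPawn at the origin, the next four get BP_PlayerCharacter in a rotated, offset row.
; Each valid spawn is possessed and increments the index.
; A branch shrinking non-VR pawns is left disconnected.
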(event `self.K2_PostLogin`
  (params (NewPlayer :type "PlayerController Object Reference"))
  (bind _returnvalue (`KismetMathLibrary.MakeTransform` (`KismetMathLibrary.MakeVector` 450.0 (* (`self.PlayerIndex`) 50.0)) (struct :`Yaw` 180.0)))
  (bind _returnvalue_2 (`|SpawnActorFromClass` (select `int` (`self.PlayerIndex`) :`0` "/Game/Blueprints/Character/VR/BP_VRPawn.BP_VRPawn_C" :`1` "/Game/Blueprints/Character/ThirdPerson/BP_PlayerCharacter.BP_PlayerCharacter_C" :`2` "/Game/Blueprints/Character/ThirdPerson/BP_PlayerCharacter.BP_PlayerCharacter_C" :`3` "/Game/Blueprints/Character/ThirdPerson/BP_PlayerCharacter.BP_PlayerCharacter_C" :`4` "/Game/Blueprints/Character/ThirdPerson/BP_PlayerCharacter.BP_PlayerCharacter_C" :!type "Actor Class Reference") (select `int` (`self.PlayerIndex`) :`0` (`KismetMathLibrary.MakeTransform` (0.0 0.0 0.0)) :`1` _returnvalue :`2` _returnvalue :`3` _returnvalue :`4` _returnvalue) "AlwaysSpawn" "OverrideRootScale" null null))
  (bind _aspawn (cast `Pawn` _returnvalue_2))
  (`/Engine/EditorBlueprintResources/StandardMacros.IsValid` _aspawn
    (:`Is Valid`
      (`Controller.Possess` NewPlayer _aspawn)
      (`/Engine/EditorBlueprintResources/StandardMacros.IncrementInt` (`self.PlayerIndex`)))))

(fn `UserConstructionScript`)