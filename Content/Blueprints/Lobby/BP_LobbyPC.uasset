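; Lobby player controller that shows the lobby UI and moves the session into the main game map.
; On BeginPlay, with authority only, it creates the lobby widget and shows the mouse cursor.
; Its GameStart event waits briefly, then issues a servertravel console command for the Main map.
; A disconnected, unused branch would spawn a game-start switch in front of the VR pawn's camera and attach it there.
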(event `self.ReceiveBeginPlay`
  (`/Engine/EditorBlueprintResources/ActorMacros.Switch Has Authority`
    (:`Authority`
      (bind _returnvalue (`|CreateWidget` "/Game/Blueprints/Lobby/LobbyWidget.LobbyWidget_C"))
      (`UserWidget.AddToViewport` _returnvalue 0)
      (set `self.bShowMouseCursor` true))))

(event `GameStart`
  (`KismetSystemLibrary.PrintString` "GameStart")
  (`KismetSystemLibrary.Delay` 2.0)
  (`KismetSystemLibrary.ExecuteConsoleCommand` "servertravel/Game/Maps/Main" null))

(fn `UserConstructionScript`)